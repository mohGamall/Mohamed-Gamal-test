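; Test actor Blueprint that exercises a custom event-object system with typed key-value payloads, shared between Blueprint and C++.
; After a short delay on BeginPlay, it binds to a C++ event, whose handler prints damage details for TakeDamage events.
; It then builds two Blueprint events, a random home location (never triggered) and a door opening (triggered), printing their data.
; The door branch finally triggers the C++ event.
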(event Custom|When%20Event%20Triggered
  (params (TriggeredEvent :type Event%20Object%20Reference))
  ;[0.04706 1 0.07059] Subscription Example for an event from CPP
  (if (Utilities|Enum|Equal(Enum) (Class|Event|GetEventType TriggeredEvent) "TakeDamage")
    (Development|PrintString (Utilities|String|Append "Awwww that hurt, Damage Taken is :  " (Utilities|String|ToString(Integer) (Utilities|Struct|BreakEventData (.RetValue (Class|Event|GetData TriggeredEvent "Damage")))) " " (Utilities|Struct|BreakEventData (.RetValue (Class|Event|GetData TriggeredEvent "DamageDealerName"))) " Did this !") true true "(R=1.000000,G=0.006141,B=0.000000,A=1.000000)" 99.0)))

(event EventBeginPlay
  (|CallParentFunction)
  ;[0.04706 1 0.07059] Bind To Event trigger from C++
  (Utilities|FlowControl|Delay 1.0)
  (EventDispatchers|BindEventtoOnEventTriggered (Variables|Default|GetEventCPP) (EventDispatchers|CreateEvent :!event Custom|When%20Event%20Triggered))
  (Utilities|FlowControl|Sequence
    (:then_0
      ;[0.3707 1 0.7436] Creating Custom Event and setting its data
      (bind _returnvalue (Game|ConstructObjectfromClass "/Game/BPS/Event_BP.Event_BP_C"))
      (Variables|Default|SetEvent_Inst _returnvalue)
      (Class|Event|SetEventType (Variables|Default|GetEvent_Inst) "CustomEvent")
      (Class|Event|AddData (Variables|Default|GetEvent_Inst) "EventName" (Utilities|Struct|MakeEventData "SetHomeLocation"))
      (Class|Event|AddData (Variables|Default|GetEvent_Inst) "Home Location" (Utilities|Struct|MakeEventData (Math|Vector|MakeVector (Math|Random|RandomFloatinRange -1e+04 1e+04) (Math|Random|RandomFloatinRange -1e+04 1e+04) (Math|Random|RandomFloatinRange -1e+04 1e+04))))
      (Development|PrintString "this data is done in TestActror Blueprint" true true "(R=0.000000,G=0.660000,B=1.000000,A=1.000000)" 99.0)
      (Development|PrintString (Utilities|String|Append "Home Location : " (Utilities|String|ToString(Vector) (Utilities|Struct|BreakEventData (.RetValue (Class|Event|GetData (Variables|Default|GetEvent_Inst) "Home Location"))))) true true "(R=1.000000,G=0.627254,B=0.000000,A=1.000000)" 999.0))
    (:then_1
      ;[0.2474 0.3933 1] Making an event for Door Openeing
      (bind _returnvalue_2 (Game|ConstructObjectfromClass "/Game/BPS/Event_BP.Event_BP_C"))
      (Variables|Default|SetOpenDoorEvent _returnvalue_2)
      (Class|Event|SetEventType (Variables|Default|GetOpenDoorEvent) "OpenDoor")
      (Class|Event|AddData (Variables|Default|GetOpenDoorEvent) "DoorID" (Utilities|Struct|MakeEventData "Int" 949))
      (Class|Event|AddData (Variables|Default|GetOpenDoorEvent) "IsOpen" (Utilities|Struct|MakeEventData "Int" true))
      (Class|Event|TriggerEvent (Variables|Default|GetOpenDoorEvent))
      (if (Utilities|Enum|Equal(Enum) (Class|Event|GetEventType (Variables|Default|GetOpenDoorEvent)) "OpenDoor")
        (Development|PrintString (Utilities|String|Append "Door " (Utilities|String|ToString(Integer) (Utilities|Struct|BreakEventData (.RetValue (Class|Event|GetData (Variables|Default|GetOpenDoorEvent) "DoorID")))) " is now " (Utilities|String|SelectString "Open" "Close" (Utilities|Struct|BreakEventData (.RetValue (Class|Event|GetData (Variables|Default|GetOpenDoorEvent) "IsOpen"))))) true true "(R=0.000000,G=0.660000,B=1.000000,A=1.000000)" 99.0)
        (Class|Event|TriggerEvent (Variables|Default|GetEventCPP))))))

(fn ConstructionScript)